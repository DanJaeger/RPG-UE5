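; Anim notify state that opens and closes the sword trace window during an animation.
; On begin it starts the trace and on end it stops it, based on who owns the mesh.
; For BP_ThirdPersonCharacter the calls go to its BPCAttackSystem component, while BP_AI_Generic receives them on the actor itself.
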(fn ReceivedNotifyBegin
  (params (MeshComp :type Skeletal%20Mesh%20Component%20Object%20Reference) (Animation :type Anim%20Sequence%20Base%20Object%20Reference) (TotalDuration :type Float%20%28single-precision%29) (EventReference :type Anim%20Notify%20Event%20Reference%20Structure%20%28by%20ref%29))
  (bind _returnvalue (Components|GetOwner MeshComp))
  (bind _asbp_third_person_character (Utilities|Casting|CastToBP_ThirdPersonCharacter _returnvalue)
    (:then
      (Default|StartSwordTrace (Variables|/Game/Blueprints/Characters/BP_ThirdPersonCharacter.BP_ThirdPersonCharacter_C|GetBPC_AttackSystem _asbp_third_person_character)))
    (:CastFailed
      (bind _asbp_ai_generic (Utilities|Casting|CastToBP_AI_Generic _returnvalue))
      (Default|StartSwordTrace _asbp_ai_generic)))
  (return false))

(fn ReceivedNotifyEnd
  (params (MeshComp :type Skeletal%20Mesh%20Component%20Object%20Reference) (Animation :type Anim%20Sequence%20Base%20Object%20Reference) (EventReference :type Anim%20Notify%20Event%20Reference%20Structure%20%28by%20ref%29))
  (bind _returnvalue (Components|GetOwner MeshComp))
  (bind _asbp_third_person_character (Utilities|Casting|CastToBP_ThirdPersonCharacter _returnvalue)
    (:then
      (Default|StopSwordTrace (Variables|/Game/Blueprints/Characters/BP_ThirdPersonCharacter.BP_ThirdPersonCharacter_C|GetBPC_AttackSystem _asbp_third_person_character)))
    (:CastFailed
      (bind _asbp_ai_generic (Utilities|Casting|CastToBP_AI_Generic _returnvalue))
      (Default|StopSwordTrace _asbp_ai_generic)))
  (return false))