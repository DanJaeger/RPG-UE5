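; Actor component that tracks health, stamina, XP and level, attached to the player character, training dummy or generic AI.
; BeginPlay casts the owner to cache a typed reference for updating HUD or DummyUI bars directly.
; Damage and stamina functions return death or remaining-stamina flags, and regained stamina re-enables sprinting.
; Reaching max XP levels up, resetting XP, raising the threshold and playing a sound.
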(event EventBeginPlay
  (bind _returnvalue (Components|GetOwner))
  ;[0.05127 0.05127 0.05127] Cast Player
  (bind _asbp_third_person_character (Utilities|Casting|CastToBP_ThirdPersonCharacter (Components|GetOwner))
    (:then
      (Variables|Default|SetPlayerCharacterBP _asbp_third_person_character)
      (Variables|Default|SetIsPlayer true))
    (:CastFailed
      (bind _asbp_dummy (Utilities|Casting|CastToBP_Dummy _returnvalue)
        (:then
          (Variables|Default|SetDummyBP _asbp_dummy))
        (:CastFailed
          (bind _asbp_ai_generic (Utilities|Casting|CastToBP_AI_Generic _returnvalue))
          (Variables|Default|SetBP%20AI%20Generic _asbp_ai_generic)
          (Variables|Default|SetIsPlayer false))))))

(fn DecreaseHealth
  (params (Damage :type Float%20%28double-precision%29))
  (if (> (Variables|Health|GetCurrentHealth) 0.0)
    (bind _output_get (Variables|Health|SetCurrentHealth (- (Variables|Health|GetCurrentHealth) Damage)))
    (bind _dummybp (Variables|Default|GetDummyBP)
      (:then
        (Progress|SetPercent (Variables|/Game/UI/HUD/WB_Dummy_HUD.WB_Dummy_HUD_C|GetHealthBar (Variables|/Game/Blueprints/Characters/BP_AI_Generic.BP_AI_Generic_C|GetDummyUI (stale _bp_ai_generic))) (/ _output_get (Variables|Health|GetMaxHealth)) :!label _label))
      (:else
        (bind _bp_ai_generic (Variables|Default|GetBP%20AI%20Generic)
          (:then
            (goto _label))
          (:else
            (Development|PrintString "AQUI")
            (Progress|SetPercent (select (Variables|Default|GetIsPlayer) (Variables|/Game/UI/HUD/WB_HUD.WB_HUD_C|GetHealthBar (Variables|/Game/Blueprints/Characters/BP_ThirdPersonCharacter.BP_ThirdPersonCharacter_C|GetHUD%20Widget (Variables|Default|GetPlayerCharacterBP))) (Variables|/Game/UI/HUD/WB_Dummy_HUD.WB_Dummy_HUD_C|GetHealthBar (Variables|/Game/Blueprints/Characters/BP_Dummy.BP_Dummy_C|GetDummyUI _dummybp))) (/ _output_get (Variables|Health|GetMaxHealth)))))))
    (if (<= (Variables|Health|GetCurrentHealth) 0.0)
      _
      (else
        (return false))))
  (return true))

(fn IncreaseMaxHealth
  (params (Increment :type Float%20%28double-precision%29))
  (Variables|Health|SetMaxHealth (+ (Variables|Health|GetMaxHealth) Increment))
  (Progress|SetPercent (Variables|/Game/UI/HUD/WB_HUD.WB_HUD_C|GetHealthBar (Variables|/Game/Blueprints/Characters/BP_ThirdPersonCharacter.BP_ThirdPersonCharacter_C|GetHUD%20Widget (Variables|Default|GetPlayerCharacterBP))) (/ (Variables|Health|GetCurrentHealth) (Variables|Health|GetMaxHealth))))

(fn DecreaseStamina
  (params (StaminaDepleted :type Float%20%28double-precision%29))
  (if (> (Variables|Stamina|GetCurrentStamina) 0.0)
    (Variables|Stamina|SetCurrentStamina (- (Variables|Stamina|GetCurrentStamina) StaminaDepleted))
    (Progress|SetPercent (Variables|/Game/UI/HUD/WB_HUD.WB_HUD_C|GetStaminaBar (Variables|/Game/Blueprints/Characters/BP_ThirdPersonCharacter.BP_ThirdPersonCharacter_C|GetHUD%20Widget (Variables|Default|GetPlayerCharacterBP))) (/ (Variables|Stamina|GetCurrentStamina) (Variables|Stamina|GetMaxStamina)))
    (if (<= (Variables|Stamina|GetCurrentStamina) 0.0)
      _
      (else
        (return true))))
  (return false))

(fn IncreaseMaxStamina
  (params (StaminaGained :type Float%20%28double-precision%29))
  (Variables|Stamina|SetMaxStamina (+ (Variables|Stamina|GetMaxStamina) StaminaGained))
  (Progress|SetPercent (Variables|/Game/UI/HUD/WB_HUD.WB_HUD_C|GetStaminaBar (Variables|/Game/Blueprints/Characters/BP_ThirdPersonCharacter.BP_ThirdPersonCharacter_C|GetHUD%20Widget (Variables|Default|GetPlayerCharacterBP))) (/ (Variables|Stamina|GetCurrentStamina) (Variables|Stamina|GetMaxStamina))))

(fn IncreaseHealth
  (params (Health%20Gained :type Float%20%28double-precision%29))
  (Variables|Health|SetCurrentHealth (+ (Variables|Health|GetCurrentHealth) Health%20Gained))
  (if (> (Variables|Health|GetCurrentHealth) (Variables|Health|GetMaxHealth))
    (Variables|Health|SetCurrentHealth (Variables|Health|GetMaxHealth)))
  (Progress|SetPercent (Variables|/Game/UI/HUD/WB_HUD.WB_HUD_C|GetHealthBar (Variables|/Game/Blueprints/Characters/BP_ThirdPersonCharacter.BP_ThirdPersonCharacter_C|GetHUD%20Widget (Variables|Default|GetPlayerCharacterBP))) (/ (Variables|Health|GetCurrentHealth) (Variables|Health|GetMaxHealth))))

(fn IncreaseStamina
  (params (Stamina%20Gained :type Float%20%28double-precision%29))
  (Variables|Stamina|SetCurrentStamina (+ (Variables|Stamina|GetCurrentStamina) Stamina%20Gained))
  (if (> (Variables|Stamina|GetCurrentStamina) (Variables|Stamina|GetMaxStamina))
    (Variables|Stamina|SetCurrentStamina (Variables|Stamina|GetMaxStamina)))
  (Progress|SetPercent (Variables|/Game/UI/HUD/WB_HUD.WB_HUD_C|GetStaminaBar (Variables|/Game/Blueprints/Characters/BP_ThirdPersonCharacter.BP_ThirdPersonCharacter_C|GetHUD%20Widget (Variables|Default|GetPlayerCharacterBP))) (/ (Variables|Stamina|GetCurrentStamina) (Variables|Stamina|GetMaxStamina)))
  (if (> (Variables|Stamina|GetCurrentStamina) 0.0)
    (Variables|/Game/Blueprints/Characters/BP_ThirdPersonCharacter.BP_ThirdPersonCharacter_C|SetCanSprint (Variables|Default|GetPlayerCharacterBP) true)))

(fn InitPlayerData
  (Progress|SetPercent (Variables|/Game/UI/HUD/WB_HUD.WB_HUD_C|GetStaminaBar (Variables|/Game/Blueprints/Characters/BP_ThirdPersonCharacter.BP_ThirdPersonCharacter_C|GetHUD%20Widget (Variables|Default|GetPlayerCharacterBP))) (/ (Variables|Stamina|GetCurrentStamina) (Variables|Stamina|GetMaxStamina)))
  (Progress|SetPercent (Variables|/Game/UI/HUD/WB_HUD.WB_HUD_C|GetHealthBar (Variables|/Game/Blueprints/Characters/BP_ThirdPersonCharacter.BP_ThirdPersonCharacter_C|GetHUD%20Widget (Variables|Default|GetPlayerCharacterBP))) (/ (Variables|Health|GetCurrentHealth) (Variables|Health|GetMaxHealth)))
  (Progress|SetPercent (Variables|/Game/UI/HUD/WB_HUD.WB_HUD_C|GetXpBar (Variables|/Game/Blueprints/Characters/BP_ThirdPersonCharacter.BP_ThirdPersonCharacter_C|GetHUD%20Widget (Variables|Default|GetPlayerCharacterBP))) (/ (Variables|XP|GetXP) (Variables|XP|GetMaxXP)))
  (Rendering|Components|TextRender|SetText (Variables|/Game/UI/HUD/WB_HUD.WB_HUD_C|GetPlayerXPText (Variables|/Game/Blueprints/Characters/BP_ThirdPersonCharacter.BP_ThirdPersonCharacter_C|GetHUD%20Widget (Variables|Default|GetPlayerCharacterBP))) (Utilities|Text|FormatText "{CurrentXP} / {MaxXP}" (Variables|XP|GetXP) (Variables|XP|GetMaxXP)))
  (Rendering|Components|TextRender|SetText (Variables|/Game/UI/HUD/WB_HUD.WB_HUD_C|GetPlayerLevelText (Variables|/Game/Blueprints/Characters/BP_ThirdPersonCharacter.BP_ThirdPersonCharacter_C|GetHUD%20Widget (Variables|Default|GetPlayerCharacterBP))) (Utilities|Text|ToText(Integer) (Variables|XP|GetLevel))))

(fn IncreaseXP
  (params (XP%20Gained :type Float%20%28double-precision%29))
  (Variables|XP|SetXP (+ (Variables|XP|GetXP) XP%20Gained))
  (if (>= (Variables|XP|GetXP) (Variables|XP|GetMaxXP))
    (LevelandXP|IncreaseLevel))
  (Progress|SetPercent (Variables|/Game/UI/HUD/WB_HUD.WB_HUD_C|GetXpBar (Variables|/Game/Blueprints/Characters/BP_ThirdPersonCharacter.BP_ThirdPersonCharacter_C|GetHUD%20Widget (Variables|Default|GetPlayerCharacterBP))) (/ (Variables|XP|GetXP) (Variables|XP|GetMaxXP)))
  (Rendering|Components|TextRender|SetText (Variables|/Game/UI/HUD/WB_HUD.WB_HUD_C|GetPlayerXPText (Variables|/Game/Blueprints/Characters/BP_ThirdPersonCharacter.BP_ThirdPersonCharacter_C|GetHUD%20Widget (Variables|Default|GetPlayerCharacterBP))) (Utilities|Text|FormatText "{CurrentXP} / {MaxXP}" (Variables|XP|GetXP) (Variables|XP|GetMaxXP))))

(fn IncreaseLevel
  (Variables|XP|SetLevel (+ (Variables|XP|GetLevel) 1))
  (Variables|XP|SetMaxXP (+ (Variables|XP|GetMaxXP) 1.5e+02))
  (Variables|XP|SetXP 0.0)
  (Rendering|Components|TextRender|SetText (Variables|/Game/UI/HUD/WB_HUD.WB_HUD_C|GetPlayerLevelText (Variables|/Game/Blueprints/Characters/BP_ThirdPersonCharacter.BP_ThirdPersonCharacter_C|GetHUD%20Widget (Variables|Default|GetPlayerCharacterBP))) (Utilities|Text|ToText(Integer) (Variables|XP|GetLevel)))
  (Audio|PlaySound2D "/Game/Sounds/UI/LevelUp.LevelUp" 1.0 1.0 0.0 0 0))

(fn InitDummyData
  (bind _dummybp (Variables|Default|GetDummyBP)
    (:then
      (Progress|SetPercent (Variables|/Game/UI/HUD/WB_Dummy_HUD.WB_Dummy_HUD_C|GetHealthBar (Variables|/Game/Blueprints/Characters/BP_Dummy.BP_Dummy_C|GetDummyUI _dummybp)) (/ (Variables|Health|GetCurrentHealth) (Variables|Health|GetMaxHealth))))
    (:else
      (bind _bp_ai_generic (Variables|Default|GetBP%20AI%20Generic)
        (:then
          (Progress|SetPercent (Variables|/Game/UI/HUD/WB_Dummy_HUD.WB_Dummy_HUD_C|GetHealthBar (Variables|/Game/Blueprints/Characters/BP_AI_Generic.BP_AI_Generic_C|GetDummyUI _bp_ai_generic)) (/ (Variables|Health|GetCurrentHealth) (Variables|Health|GetMaxHealth))))
        (:else)))))