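; Actor component that gives the third-person player ledge climbing: grab, shimmy, side hop and drop or hang down.
; Chained sphere traces from character tracer components find walls, ledge points, gaps and hang-down edges.
; SetOnWall disables capsule collision, switches to Flying, plays montages and moves the capsule into place; a foot trace picks OnLedge or Hanging.
; Falling auto-grab is unfinished: Tick calls an empty event.
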(event Custom|E_GrabLedge
  ;[0.05127 0.05127 0.05127] Grab Ledge
  (Utilities|GrabLedge))

(event Custom|E_DropDown
  (Utilities|DropDown)
  (Variables|Default|SetCheckHopLeft false)
  (Variables|Default|SetCheckHopRight false))

(event Custom|E_CheckToHop
  (Utilities|HopLedge))

(event Custom|E_AutoGrabLedge
  ;[0.05127 0.05127 0.05127] Grab Ledge While Falling
)

(event EventBeginPlay
  ;[0.05127 0.05127 0.05127] Initializing Player Components
  (bind _asbp_third_person_character (Utilities|Casting|CastToBP_ThirdPersonCharacter (Game|GetPlayerCharacter 0)))
  (Variables|References|SetPlayerRef _asbp_third_person_character)
  (Utilities|FlowControl|Sequence
    (:then_0
      (Variables|Default|SetPlayerMovement (Variables|/Script/Engine.Character|GetCharacterMovement (Variables|References|GetPlayerRef))))
    (:then_1
      (Variables|Default|SetPlayerCapsuleComp (Variables|/Script/Engine.Character|GetCapsuleComponent (Variables|References|GetPlayerRef))))
    (:then_2
      (Variables|Default|SetPlayerMesh (Variables|/Script/Engine.Character|GetMesh (Variables|References|GetPlayerRef))))
    (:then_3
      (Variables|References|SetAnimRef (Components|SkeletalMesh|GetAnimInstance (Variables|Default|GetPlayerMesh))))))

(event EventTick
  (params (DeltaSeconds :type Float%20%28single-precision%29))
  (switch Utilities|FlowControl|Switch|SwitchonEMovementMode (Variables|/Script/Engine.CharacterMovementComponent|GetMovementMode (Variables|Default|GetPlayerMovement))
    (:MOVE_Falling
      (CallFunction|EAutoGrabLedge))))

(fn GetWallLocation
  (bind _playerref (Variables|References|GetPlayerRef))
  (bind _frontwalltracer (Variables|/Game/Blueprints/Characters/BP_ThirdPersonCharacter.BP_ThirdPersonCharacter_C|GetFrontWallTracer _playerref))
  (bind _returnvalue (Transformation|GetWorldLocation _frontwalltracer))
  (bind (_outhit _returnvalue_2) (Collision|SphereTraceByChannel _returnvalue (+ _returnvalue (* (Math|Vector|GetForwardVector (Transformation|GetWorldRotation _frontwalltracer)) 1e+02)) 1e+01 "TraceTypeQuery3" false 0 "ForOneFrame" true "(R=1.000000,G=0.000000,B=0.000000,A=1.000000)" "(R=0.109804,G=1.000000,B=0.117647,A=1.000000)")) ; Check for wall in front
  (if _returnvalue_2
    (Variables|Default|SetWallImpactNormal (.ImpactNormal (Collision|BreakHitResult _outhit)))
    (Variables|Default|SetWallImpactPoint (.ImpactPoint (Collision|BreakHitResult _outhit)))
    (Variables|Default|SetClimbRotation (Math|Rotator|Delta(Rotator) (Math|Rotator|MakeRotfromX (.ImpactNormal (Collision|BreakHitResult _outhit))) "0.000000,180.000000,0.000000"))
    (CallFunction|GetWallHeight (.ImpactPoint (Collision|BreakHitResult _outhit)) (Transformation|GetActorForwardVector (Variables|References|GetPlayerRef)))
    (else
      (Variables|Default|SetClimbingState (Utilities|Struct|MakeBPS_ClimbingState false false))))
  (return))

(fn GetWallHeight
  (params (WallImpactPoint :type Vector) (DirectionVector :type Vector))
  (bind _climbrotation (Variables|Default|GetClimbRotation))
  (bind _ledgeheightlocationxy (Variables|Default|GetLedgeHeightLocationXY))
  (bind _returnvalue (Math|Vector|GetForwardVector _climbrotation))
  (bind _returnvalue_2 (* _returnvalue _ledgeheightlocationxy))
  (bind _returnvalue_3 (- WallImpactPoint _returnvalue_2))
  (bind (_outhit _returnvalue_4) (Collision|SphereTraceByChannel (+ WallImpactPoint (Math|Vector|MakeVector 0.0 0.0 (Variables|Default|GetWallHeightUpTraceLimit))) (+ WallImpactPoint (Math|Vector|MakeVector 0.0 0.0 (Variables|Default|GetWallHeightDownTraceLimit))) 1e+01 "TraceTypeQuery3" false 0 "ForOneFrame" true "(R=1.000000,G=0.000000,B=0.000000,A=1.000000)" "(R=0.220451,G=1.000000,B=0.092793,A=1.000000)")) ; Get Ledge Height
  (if _returnvalue_4
    (Variables|Default|SetLedgeLocation (Math|Vector|MakeVector (.x _returnvalue_3) (.y _returnvalue_3) (.z (- (.ImpactPoint (Collision|BreakHitResult _outhit)) (Variables|Default|GetLedgeHeightLocationZ)))))
    (bind _returnvalue_5 (Collision|SphereTraceByChannel (+ (.ImpactPoint (Collision|BreakHitResult _outhit)) "0.000000,0.000000,10.000000") (+ (.ImpactPoint (Collision|BreakHitResult _outhit)) "0.000000,0.000000,10.000000" (* DirectionVector 1e+01)) 5.0 "TraceTypeQuery3" false 0 "ForOneFrame" true "(R=1.000000,G=0.000000,B=0.000000,A=1.000000)" "(R=1.000000,G=0.156314,B=0.959148,A=1.000000)")) ; Get ledge contact point
    (Variables|Default|SetClimbingState (Utilities|Struct|MakeBPS_ClimbingState (not _returnvalue_5) false))
    (return)))

(fn LedgeMoveRight
  (bind _playerref (Variables|References|GetPlayerRef))
  (bind _rightmovetracer (Variables|/Game/Blueprints/Characters/BP_ThirdPersonCharacter.BP_ThirdPersonCharacter_C|GetRightMoveTracer _playerref))
  (bind _returnvalue (Transformation|GetWorldLocation _rightmovetracer))
  (bind (_outhit _returnvalue_2) (Collision|SphereTraceByChannel _returnvalue (+ _returnvalue (* (Math|Vector|GetForwardVector (Transformation|GetWorldRotation _rightmovetracer)) 5e+01)) 1e+01 "TraceTypeQuery3" false 0 "None")) ; Detects Ledge on the right
  (if _returnvalue_2
    (Class|BPIAnimUp|MoveonLedge(Message) (Variables|References|GetAnimRef) false true)
    (bind (_outhit_2 _returnvalue_3) (Collision|SphereTraceByChannel (+ (.ImpactPoint (Collision|BreakHitResult _outhit)) "0.000000,0.000000,20.000000") (.ImpactPoint (Collision|BreakHitResult _outhit)) 1e+01 "TraceTypeQuery3" false 0 "None"))
    (if _returnvalue_3
      (Variables|Default|SetCheckLedgeToHopImpactPointLeft/Right (.ImpactPoint (Collision|BreakHitResult _outhit_2)))
      (bind _returnvalue_4 (Collision|SphereTraceByChannel (+ (.ImpactPoint (Collision|BreakHitResult _outhit_2)) (* (Transformation|GetActorRightVector (Variables|References|GetPlayerRef)) 28.0)) (+ (.ImpactPoint (Collision|BreakHitResult _outhit_2)) (* (Transformation|GetActorRightVector (Variables|References|GetPlayerRef)) 28.0)) 1e+01 "TraceTypeQuery3" false 0 "None")) ; Detects if we keep can moving to the right
      (if _returnvalue_4
        (CallFunction|MoveonLedge (.ImpactPoint (Collision|BreakHitResult _outhit)) (.ImpactPoint (Collision|BreakHitResult _outhit_2)) (Math|Rotator|MakeRotfromX (.ImpactNormal (Collision|BreakHitResult _outhit))))
        (Variables|Default|SetCheckHopLeft false)
        (Variables|Default|SetCheckHopRight false)
        (elif (Variables|Default|GetCanMove)
          (Class|BPIAnimUp|MoveonLedge(Message) (Variables|References|GetAnimRef) false false)
          (Variables|Default|SetCheckHopRight true)
          (CallFunction|EChecktoHop)
          (return))))
    (else
      (Class|BPIAnimUp|MoveonLedge(Message) (Variables|References|GetAnimRef) false false))))

(fn MoveonLedge
  (params (Trace1%20Impact%20Point :type Vector) (Trace2%20Impact%20Point :type Vector) (Rotation :type Rotator))
  (bind _returnvalue (Math|Vector|GetForwardVector Rotation))
  (bind _returnvalue_2 (Utilities|Time|GetWorldDeltaSeconds))
  (bind (_roll _pitch _yaw) (Math|Rotator|BreakRotator Rotation))
  (bind _ledgeheightlocationxy (Variables|Default|GetLedgeHeightLocationXY))
  (bind _returnvalue_3 (* _returnvalue _ledgeheightlocationxy))
  (bind _returnvalue_4 (+ Trace1%20Impact%20Point _returnvalue_3))
  (Transformation|SetActorLocationAndRotation (Variables|References|GetPlayerRef) (Math|Interpolation|VInterpTo (Transformation|GetActorLocation (Variables|References|GetPlayerRef)) (Math|Vector|MakeVector (.x _returnvalue_4) (.y _returnvalue_4) (- (.Z (Math|Vector|BreakVector Trace2%20Impact%20Point)) (Variables|Default|GetLedgeHeightLocationZ))) _returnvalue_2 2.0) (Math|Interpolation|RInterpTo (Transformation|GetActorRotation (Variables|References|GetPlayerRef)) (Math|Rotator|MakeRotator _roll _pitch (- _yaw 1.8e+02)) _returnvalue_2 5.0))
  (return))

(fn LedgeMoveLeft
  (bind _playerref (Variables|References|GetPlayerRef))
  (bind _leftmovetracer (Variables|/Game/Blueprints/Characters/BP_ThirdPersonCharacter.BP_ThirdPersonCharacter_C|GetLeftMoveTracer _playerref))
  (bind _returnvalue (Transformation|GetWorldLocation _leftmovetracer))
  (bind (_outhit _returnvalue_2) (Collision|SphereTraceByChannel _returnvalue (+ _returnvalue (* (Math|Vector|GetForwardVector (Transformation|GetWorldRotation _leftmovetracer)) 5e+01)) 1e+01 "TraceTypeQuery3" false 0 "None")) ; Detects Ledge on the right
  (if _returnvalue_2
    (Class|BPIAnimUp|MoveonLedge(Message) (Variables|References|GetAnimRef) true false)
    (bind (_outhit_2 _returnvalue_3) (Collision|SphereTraceByChannel (+ (.ImpactPoint (Collision|BreakHitResult _outhit)) "0.000000,0.000000,20.000000") (.ImpactPoint (Collision|BreakHitResult _outhit)) 1e+01 "TraceTypeQuery3" false 0 "None"))
    (if _returnvalue_3
      (Variables|Default|SetCheckLedgeToHopImpactPointLeft/Right (.ImpactPoint (Collision|BreakHitResult _outhit_2)))
      (bind _returnvalue_4 (Collision|SphereTraceByChannel (+ (.ImpactPoint (Collision|BreakHitResult _outhit_2)) (* (Transformation|GetActorRightVector (Variables|References|GetPlayerRef)) -28.0)) (+ (.ImpactPoint (Collision|BreakHitResult _outhit_2)) (* (Transformation|GetActorRightVector (Variables|References|GetPlayerRef)) -28.0)) 1e+01 "TraceTypeQuery3" false 0 "None")) ; Detects if we can keep moving to the right
      (if _returnvalue_4
        (CallFunction|MoveonLedge (.ImpactPoint (Collision|BreakHitResult _outhit)) (.ImpactPoint (Collision|BreakHitResult _outhit_2)) (Math|Rotator|MakeRotfromX (.ImpactNormal (Collision|BreakHitResult _outhit))))
        (Variables|Default|SetCheckHopRight false)
        (Variables|Default|SetCheckHopLeft false)
        (elif (Variables|Default|GetCanMove)
          (Class|BPIAnimUp|MoveonLedge(Message) (Variables|References|GetAnimRef) false false)
          (Variables|Default|SetCheckHopLeft true)
          (CallFunction|EChecktoHop)
          (return))))
    (else
      (Class|BPIAnimUp|MoveonLedge(Message) (Variables|References|GetAnimRef) false false))))

(fn TraceFeetonWall
  (bind _playerref (Variables|References|GetPlayerRef))
  (bind _mesh (Variables|/Script/Engine.Character|GetMesh _playerref))
  (bind _returnvalue (Transformation|GetSocketLocation _mesh "foot_l"))
  (bind _returnvalue_2 (Collision|MultiLineTraceByChannel _returnvalue (+ _returnvalue (* (Transformation|GetActorForwardVector (Variables|References|GetPlayerRef)) 2e+01)) "TraceTypeQuery1" false 0 "ForDuration"))
  (return _returnvalue_2))