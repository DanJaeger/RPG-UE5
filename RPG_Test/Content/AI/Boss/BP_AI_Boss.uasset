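; BP_AI_Boss is the boss AI actor, adding a health sync to the behavior it inherits from its parent.
; Every Tick, after the parent's Tick, it casts its controller to BP_AIController_Boss and copies current and max health from BPPlayerStats into it.
; The controller is updated by per-frame polling, and the construction script only calls the parent.
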(event EventBeginPlay
  (|CallParentFunction) ; This node is disabled and will not be called.\nDrag off pins to build functionality.
)

(event Collision|EventActorBeginOverlap
  (params (OtherActor :type Actor%20Object%20Reference)))

(event EventTick
  (params (DeltaSeconds :type Float%20%28single-precision%29))
  (|CallParentFunction DeltaSeconds)
  (bind _asbp_aicontroller_boss (Utilities|Casting|CastToBP_AIController_Boss (AI|GetAIController self)))
  (Variables|/Game/AI/Boss/BP_AIController_Boss.BP_AIController_Boss_C|SetHealth _asbp_aicontroller_boss (Variables|/Game/Blueprints/BP_PlayerStats.BP_PlayerStats_C|GetCurrentHealth (Variables|Default|GetBP_PlayerStats)))
  (Variables|/Game/AI/Boss/BP_AIController_Boss.BP_AIController_Boss_C|SetMaxHealth _asbp_aicontroller_boss (Variables|/Game/Blueprints/BP_PlayerStats.BP_PlayerStats_C|GetMaxHealth (Variables|Default|GetBP_PlayerStats))))

(fn ConstructionScript
  (|CallParentFunction))