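; Generic AI controller that runs the BT_AI behavior tree and feeds it sight and hearing perception through Blackboard keys.
; Sight sets TargetActor and, for boss controllers, starts boss combat; lost sight or any non-sight stimulus clears the target and ends boss combat.
; Hearing stores the stimulus location as InvestigationLocation and calls the investigation icon toggle on the controlled BP_AI_Generic pawn.
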(event OnTargetPerceptionUpdated(AIPerception)
  (params (Actor :type Actor%20Object%20Reference) (Stimulus :type AI%20Stimulus%20Structure))
  ;[0.05127 0.05127 0.05127] Detect Target / Investigate Targets
  (CallFunction|SightDetection Actor Stimulus)
  (CallFunction|HearingDetection Actor Stimulus))

(event EventBeginPlay
  (AI|RunBehaviorTree "/Game/AI/BehaviorTrees/BT_AI.BT_AI"))

(fn ConstructionScript)

(fn SightDetection
  (params (Actor :type Actor%20Object%20Reference) (Stimulus :type AI%20Stimulus%20Structure))
  (bind _returnvalue (Class|AIPerceptionSystem|GetSenseClassforStimulus Stimulus))
  (if (== _returnvalue "/Script/AIModule.AISense_Sight")
    (if (.bSuccessfullySensed (Utilities|Struct|BreakAIStimulus Stimulus))
      (AI|Components|Blackboard|SetValueasObject (AI|GetBlackboard 0) (Utilities|Name|MakeLiteralName "TargetActor") Actor)
      (bind _asbp_aicontroller_boss (Utilities|Casting|CastToBP_AIController_Boss self))
      (Default|ActivateBossCombat _asbp_aicontroller_boss)
      (else
        (AI|Components|Blackboard|SetValueasObject (AI|GetBlackboard 0) (Utilities|Name|MakeLiteralName "TargetActor") 0 :!label _label)
        (bind _asbp_aicontroller_boss_2 (Utilities|Casting|CastToBP_AIController_Boss self))
        (Default|DeactivateBossCombat _asbp_aicontroller_boss_2)))
    (else
      (goto _label))))

(fn HearingDetection
  (params (Actor :type Actor%20Object%20Reference) (Stimulus :type AI%20Stimulus%20Structure))
  (bind _returnvalue (Class|AIPerceptionSystem|GetSenseClassforStimulus Stimulus))
  (if (== _returnvalue "/Script/AIModule.AISense_Hearing")
    (AI|Components|Blackboard|SetValueasVector (AI|GetBlackboard 0) (Utilities|Name|MakeLiteralName "InvestigationLocation") (.StimulusLocation (Utilities|Struct|BreakAIStimulus Stimulus)))
    (bind _asbp_ai_generic (Utilities|Casting|CastToBP_AI_Generic (Pawn|GetControlledPawn)))
    (Default|Enable/DisableInvestigationIcon _asbp_ai_generic)))