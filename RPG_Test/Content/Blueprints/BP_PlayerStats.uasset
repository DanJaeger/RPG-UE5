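; Player stats component for BP_ThirdPersonCharacter that tracks health, stamina, XP and level.
; Each change function updates its value and writes directly to the owner's HUD widget, with InitPlayerData refreshing the whole display.
; Decrease functions return whether health is depleted or stamina remains, and regained stamina re-enables sprinting.
; Reaching max XP levels up, resetting XP without carryover, raising the threshold and playing a sound.
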(event EventBeginPlay
  ;[0.05127 0.05127 0.05127] Cast Player
  (bind _asbp_third_person_character (Utilities|Casting|CastToBP_ThirdPersonCharacter (Components|GetOwner)))
  (Variables|Default|SetPlayerCharacterBP _asbp_third_person_character))

(fn DecreaseHealth
  (params (Damage :type Float%20%28double-precision%29))
  (if (> (Variables|Health|GetCurrentHealth) 0.0)
    (bind _output_get (Variables|Health|SetCurrentHealth (- (Variables|Health|GetCurrentHealth) Damage)))
    (Progress|SetPercent (Variables|/Game/UI/WB_HUD.WB_HUD_C|GetHealthBar (Variables|/Game/ThirdPerson/Blueprints/BP_ThirdPersonCharacter.BP_ThirdPersonCharacter_C|GetHUD%20Widget (Variables|Default|GetPlayerCharacterBP))) (/ _output_get (Variables|Health|GetMaxHealth)))
    (if (<= (Variables|Health|GetCurrentHealth) 0.0)
      _
      (else
        (return false))))
  (return true))

(fn IncreaseMaxHealth
  (params (Increment :type Float%20%28double-precision%29))
  (Variables|Health|SetMaxHealth (+ (Variables|Health|GetMaxHealth) Increment))
  (Progress|SetPercent (Variables|/Game/UI/WB_HUD.WB_HUD_C|GetHealthBar (Variables|/Game/ThirdPerson/Blueprints/BP_ThirdPersonCharacter.BP_ThirdPersonCharacter_C|GetHUD%20Widget (Variables|Default|GetPlayerCharacterBP))) (/ (Variables|Health|GetCurrentHealth) (Variables|Health|GetMaxHealth))))

(fn DecreaseStamina
  (params (StaminaDepleted :type Float%20%28double-precision%29))
  (if (> (Variables|Stamina|GetCurrentStamina) 0.0)
    (Variables|Stamina|SetCurrentStamina (- (Variables|Stamina|GetCurrentStamina) StaminaDepleted))
    (Progress|SetPercent (Variables|/Game/UI/WB_HUD.WB_HUD_C|GetStaminaBar (Variables|/Game/ThirdPerson/Blueprints/BP_ThirdPersonCharacter.BP_ThirdPersonCharacter_C|GetHUD%20Widget (Variables|Default|GetPlayerCharacterBP))) (/ (Variables|Stamina|GetCurrentStamina) (Variables|Stamina|GetMaxStamina)))
    (if (<= (Variables|Stamina|GetCurrentStamina) 0.0)
      _
      (else
        (return true))))
  (return false))

(fn IncreaseMaxStamina
  (params (StaminaGained :type Float%20%28double-precision%29))
  (Variables|Stamina|SetMaxStamina (+ (Variables|Stamina|GetMaxStamina) StaminaGained))
  (Progress|SetPercent (Variables|/Game/UI/WB_HUD.WB_HUD_C|GetStaminaBar (Variables|/Game/ThirdPerson/Blueprints/BP_ThirdPersonCharacter.BP_ThirdPersonCharacter_C|GetHUD%20Widget (Variables|Default|GetPlayerCharacterBP))) (/ (Variables|Stamina|GetCurrentStamina) (Variables|Stamina|GetMaxStamina))))

(fn IncreaseHealth
  (params (Health%20Gained :type Float%20%28double-precision%29))
  (Variables|Health|SetCurrentHealth (+ (Variables|Health|GetCurrentHealth) Health%20Gained))
  (if (> (Variables|Health|GetCurrentHealth) (Variables|Health|GetMaxHealth))
    (Variables|Health|SetCurrentHealth (Variables|Health|GetMaxHealth)))
  (Progress|SetPercent (Variables|/Game/UI/WB_HUD.WB_HUD_C|GetHealthBar (Variables|/Game/ThirdPerson/Blueprints/BP_ThirdPersonCharacter.BP_ThirdPersonCharacter_C|GetHUD%20Widget (Variables|Default|GetPlayerCharacterBP))) (/ (Variables|Health|GetCurrentHealth) (Variables|Health|GetMaxHealth))))

(fn IncreaseStamina
  (params (Stamina%20Gained :type Float%20%28double-precision%29))
  (Variables|Stamina|SetCurrentStamina (+ (Variables|Stamina|GetCurrentStamina) Stamina%20Gained))
  (if (> (Variables|Stamina|GetCurrentStamina) (Variables|Stamina|GetMaxStamina))
    (Variables|Stamina|SetCurrentStamina (Variables|Stamina|GetMaxStamina)))
  (Progress|SetPercent (Variables|/Game/UI/WB_HUD.WB_HUD_C|GetStaminaBar (Variables|/Game/ThirdPerson/Blueprints/BP_ThirdPersonCharacter.BP_ThirdPersonCharacter_C|GetHUD%20Widget (Variables|Default|GetPlayerCharacterBP))) (/ (Variables|Stamina|GetCurrentStamina) (Variables|Stamina|GetMaxStamina)))
  (if (> (Variables|Stamina|GetCurrentStamina) 0.0)
    (Variables|/Game/ThirdPerson/Blueprints/BP_ThirdPersonCharacter.BP_ThirdPersonCharacter_C|SetCanSprint (Variables|Default|GetPlayerCharacterBP) true)))

(fn InitPlayerData
  (Progress|SetPercent (Variables|/Game/UI/WB_HUD.WB_HUD_C|GetStaminaBar (Variables|/Game/ThirdPerson/Blueprints/BP_ThirdPersonCharacter.BP_ThirdPersonCharacter_C|GetHUD%20Widget (Variables|Default|GetPlayerCharacterBP))) (/ (Variables|Stamina|GetCurrentStamina) (Variables|Stamina|GetMaxStamina)))
  (Progress|SetPercent (Variables|/Game/UI/WB_HUD.WB_HUD_C|GetHealthBar (Variables|/Game/ThirdPerson/Blueprints/BP_ThirdPersonCharacter.BP_ThirdPersonCharacter_C|GetHUD%20Widget (Variables|Default|GetPlayerCharacterBP))) (/ (Variables|Health|GetCurrentHealth) (Variables|Health|GetMaxHealth)))
  (Progress|SetPercent (Variables|/Game/UI/WB_HUD.WB_HUD_C|GetXpBar (Variables|/Game/ThirdPerson/Blueprints/BP_ThirdPersonCharacter.BP_ThirdPersonCharacter_C|GetHUD%20Widget (Variables|Default|GetPlayerCharacterBP))) (/ (Variables|XP|GetXP) (Variables|XP|GetMaxXP)))
  (Rendering|Components|TextRender|SetText (Variables|/Game/UI/WB_HUD.WB_HUD_C|GetPlayerXPText (Variables|/Game/ThirdPerson/Blueprints/BP_ThirdPersonCharacter.BP_ThirdPersonCharacter_C|GetHUD%20Widget (Variables|Default|GetPlayerCharacterBP))) (Utilities|Text|FormatText "{CurrentXP} / {MaxXP}" (Variables|XP|GetXP) (Variables|XP|GetMaxXP)))
  (Rendering|Components|TextRender|SetText (Variables|/Game/UI/WB_HUD.WB_HUD_C|GetPlayerLevelText (Variables|/Game/ThirdPerson/Blueprints/BP_ThirdPersonCharacter.BP_ThirdPersonCharacter_C|GetHUD%20Widget (Variables|Default|GetPlayerCharacterBP))) (Utilities|Text|ToText(Integer) (Variables|XP|GetLevel))))

(fn IncreaseXP
  (params (XP%20Gained :type Float%20%28double-precision%29))
  (Variables|XP|SetXP (+ (Variables|XP|GetXP) XP%20Gained))
  (if (>= (Variables|XP|GetXP) (Variables|XP|GetMaxXP))
    (LevelandXP|IncreaseLevel))
  (Progress|SetPercent (Variables|/Game/UI/WB_HUD.WB_HUD_C|GetXpBar (Variables|/Game/ThirdPerson/Blueprints/BP_ThirdPersonCharacter.BP_ThirdPersonCharacter_C|GetHUD%20Widget (Variables|Default|GetPlayerCharacterBP))) (/ (Variables|XP|GetXP) (Variables|XP|GetMaxXP)))
  (Rendering|Components|TextRender|SetText (Variables|/Game/UI/WB_HUD.WB_HUD_C|GetPlayerXPText (Variables|/Game/ThirdPerson/Blueprints/BP_ThirdPersonCharacter.BP_ThirdPersonCharacter_C|GetHUD%20Widget (Variables|Default|GetPlayerCharacterBP))) (Utilities|Text|FormatText "{CurrentXP} / {MaxXP}" (Variables|XP|GetXP) (Variables|XP|GetMaxXP))))

(fn IncreaseLevel
  (Variables|XP|SetLevel (+ (Variables|XP|GetLevel) 1))
  (Variables|XP|SetMaxXP (+ (Variables|XP|GetMaxXP) 1.5e+02))
  (Variables|XP|SetXP 0.0)
  (Rendering|Components|TextRender|SetText (Variables|/Game/UI/WB_HUD.WB_HUD_C|GetPlayerLevelText (Variables|/Game/ThirdPerson/Blueprints/BP_ThirdPersonCharacter.BP_ThirdPersonCharacter_C|GetHUD%20Widget (Variables|Default|GetPlayerCharacterBP))) (Utilities|Text|ToText(Integer) (Variables|XP|GetLevel)))
  (Audio|PlaySound2D "/Game/Sounds/UI/LevelUp.LevelUp" 1.0 1.0 0.0 0 0))