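; Target dummy character that the player can damage or stealth-assassinate from behind.
; Hits play a random montage and sound, launch it along the player's facing and reduce health via BPPlayerStats.
; Death triggers delayed ragdoll, hides widgets, clears the player's lock-on and later disables capsule collision.
; An overlap radius shows the assassinate prompt, StealthBackAssassin plays the victim montage and returns alignment data, and Tick billboards both widgets toward the camera.
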(event OnComponentBeginOverlap(AssassinationRadius)
  (params (OverlappedComponent :type Primitive%20Component%20Object%20Reference) (OtherActor :type Actor%20Object%20Reference) (OtherComp :type Primitive%20Component%20Object%20Reference) (OtherBodyIndex :type Integer) (bFromSweep :type Boolean) (SweepResult :type Hit%20Result%20Structure%20%28by%20ref%29))
  ;[0.05127 0.05127 0.05127] Display Assasinate Widget
  (if (not (Variables|Default|GetIsPlayerDead))
    (Utilities|Casting|CastToBP_ThirdPersonCharacter OtherActor)
    (Rendering|SetVisibility (Variables|Default|GetAssassinate%20Widget) true false)))

(event OnComponentEndOverlap(AssassinationRadius)
  (params (OverlappedComponent :type Primitive%20Component%20Object%20Reference) (OtherActor :type Actor%20Object%20Reference) (OtherComp :type Primitive%20Component%20Object%20Reference) (OtherBodyIndex :type Integer))
  ;[0.05127 0.05127 0.05127] Display Assasinate Widget
  (Utilities|Casting|CastToBP_ThirdPersonCharacter OtherActor)
  (Rendering|SetVisibility (Variables|Default|GetAssassinate%20Widget) false false))

(event Custom|Ragdoll
  ;[0.05127 0.05127 0.05127] Enable Ragdoll
  (Utilities|FlowControl|Delay 2.0)
  (Physics|SetSimulatePhysics (Variables|Character|GetMesh) true)
  (Audio|PlaySoundatLocation "/Game/Sounds/Grunts-Hits/Death_1.Death_1" (Transformation|GetActorLocation) "0, 0, 0" 1.0 1.0 0.0 "/Game/Sounds/SA_Character.SA_Character" 0 0 0))

(event EventTick
  (params (DeltaSeconds :type Float%20%28single-precision%29))
  (bind _dummyhud (Variables|Default|GetDummyHUD))
  (bind _assassinate_widget (Variables|Default|GetAssassinate%20Widget))
  ;[0.05127 0.05127 0.05127] Rotate UI Towards Character
  (bind _final_rotation (CallFunction|SetUIRotation _dummyhud))
  (Transformation|SetWorldRotation _dummyhud _final_rotation false false)
  (bind _final_rotation_2 (CallFunction|SetUIRotation _assassinate_widget))
  (Transformation|SetWorldRotation _assassinate_widget _final_rotation_2 false false))

(event EventBeginPlay
  ;[0.05127 0.05127 0.05127] Create Widget
  (bind _aswb_dummy_hud (Utilities|Casting|CastToWB_Dummy_HUD (UserInterface|GetWidget (Variables|Default|GetDummyHUD))))
  (Variables|Default|SetDummyUI _aswb_dummy_hud)
  (Default|InitDummyData (Variables|Default|GetBP_PlayerStats)))

(event Game|Damage|EventAnyDamage
  (params (Damage :type Float%20%28single-precision%29) (DamageType :type Damage%20Type%20Object%20Reference) (InstigatedBy :type Controller%20Object%20Reference) (DamageCauser :type Actor%20Object%20Reference))
  (bind _hitanims (Variables|Default|GetHitAnims))
  ;[0.05127 0.05127 0.05127] Take Hit
  (if (not (Variables|Default|GetIsPlayerDead))
    (Animation|PlayAnimMontage (Utilities|Array|Get(acopy) _hitanims (Math|Random|RandomIntegerinRange 0 (- (Utilities|Array|Length _hitanims) 1))) 1.0 "None")
    (bind _asbp_third_person_character (Utilities|Casting|CastToBP_ThirdPersonCharacter (Game|GetPlayerCharacter 0)))
    (Character|LaunchCharacter (* (Math|Vector|GetForwardVector (Transformation|GetActorRotation _asbp_third_person_character)) 7e+02) false false)
    (Audio|PlaySoundatLocation "/Game/Sounds/Grunts-Hits/Death_2.Death_2" (Transformation|GetActorLocation) "0, 0, 0" 1.0 (Math|Random|RandomFloatinRange 0.8 1.2) 0.0 "/Game/Sounds/SA_Character.SA_Character" 0 0 0)
    (bind _isplayerdead (Default|DecreaseHealth (Variables|Default|GetBP_PlayerStats) Damage))
    (Variables|Default|SetIsPlayerDead _isplayerdead)
    (if _isplayerdead
      (CallFunction|Ragdoll)
      (Rendering|SetVisibility (Variables|Default|GetDummyHUD) false false)
      (Rendering|SetVisibility (Variables|Default|GetAssassinate%20Widget) false false)
      (Variables|/Game/Blueprints/Characters/BP_ThirdPersonCharacter.BP_ThirdPersonCharacter_C|SetActorToLockOn _asbp_third_person_character 0)
      (Utilities|FlowControl|Delay 2.0)
      (Collision|SetCollisionEnabled (Variables|Collision|GetCapsuleComponent) "NoCollision"))))

(fn ConstructionScript)

(fn SetUIRotation
  (params (Widget :type Widget%20Component%20Object%20Reference))
  (return (Math|Rotator|FindLookatRotation (Transformation|GetWorldLocation Widget) (Transformation|GetWorldLocation (Variables|/Script/Engine.PlayerCameraManager|GetTransformComponent (Game|GetPlayerCameraManager 0))))))

(fn StealthBackAssassin
  (Animation|PlayAnimMontage "/Game/Animations/Assassinations/Paired_Knife_Stealth_KidneyAndNeck_Vic_Montage.Paired_Knife_Stealth_KidneyAndNeck_Vic_Montage" 1.0 "None")
  (CallFunction|Ragdoll)
  (Rendering|SetVisibility (Variables|Default|GetAssassinate%20Widget) false false)
  (return (Transformation|GetWorldLocation (Variables|Default|GetAssassin%20REF)) (Transformation|GetActorRotation)))