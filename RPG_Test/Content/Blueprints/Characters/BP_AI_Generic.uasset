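; Generic melee enemy AI character that fights with sword combos and can be stealth-assassinated by the player.
; Attack calls drive a three-montage combo with input buffering, while timer-looped and one-shot sphere traces damage "Damageable" actors with sound, blood and camera shake.
; Incoming damage interrupts combos, launches the character and reduces BPPlayerStats health, ending in delayed ragdoll.
; Health, assassination and investigation widgets rotate toward the camera each tick.
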(event OnComponentBeginOverlap(AssassinationRadius)
  (params (OverlappedComponent :type Primitive%20Component%20Object%20Reference) (OtherActor :type Actor%20Object%20Reference) (OtherComp :type Primitive%20Component%20Object%20Reference) (OtherBodyIndex :type Integer) (bFromSweep :type Boolean) (SweepResult :type Hit%20Result%20Structure%20%28by%20ref%29))
  ;[0.05127 0.05127 0.05127] Display Assasinate Widget
  (if (not (Variables|Default|GetIsPlayerDead))
    (Utilities|Casting|CastToBP_ThirdPersonCharacter OtherActor)
    (Rendering|SetVisibility (Variables|Default|GetAssassinate%20Widget) true false)))

(event OnComponentEndOverlap(AssassinationRadius)
  (params (OverlappedComponent :type Primitive%20Component%20Object%20Reference) (OtherActor :type Actor%20Object%20Reference) (OtherComp :type Primitive%20Component%20Object%20Reference) (OtherBodyIndex :type Integer))
  ;[0.05127 0.05127 0.05127] Display Assasinate Widget
  (Utilities|Casting|CastToBP_ThirdPersonCharacter OtherActor)
  (Rendering|SetVisibility (Variables|Default|GetAssassinate%20Widget) false false))

(event Custom|SwordAttack
  ;[0.05127 0.05127 0.05127] Combo System
  ;;[0.05127 0.05127 0.05127] Sword Attack
  (if (Variables|Attack|GetIsAttacking)
    (Variables|Attack|SetSaveAttack true)
    (else
      (Variables|Attack|SetIsAttacking true)
      (switch int (Variables|Attack|GetAttackIndex)
        (:0
          (CallFunction|Attack1))
        (:1
          (CallFunction|Attack2))
        (:2
          (CallFunction|Attack4))))))

(event Custom|SwordAttackCombo
  ;[0.05127 0.05127 0.05127] Combo System
  ;;[0.05127 0.05127 0.05127] Combo Continue
  (if (Variables|Attack|GetSaveAttack)
    (Variables|Attack|SetSaveAttack false)
    (switch int (Variables|Attack|GetAttackIndex)
      (:0
        (CallFunction|Attack1))
      (:1
        (CallFunction|Attack2))
      (:2
        (CallFunction|Attack4)))
    (else
      (CallFunction|StopCombo))))

(event Custom|Sphere%20Trace
  (bind _sphere_trace_pos (Variables|Default|GetSphere%20Trace%20Pos))
  (bind _returnvalue (Transformation|GetWorldLocation _sphere_trace_pos))
  ;[0.05127 0.05127 0.05127] Sphere Trace (Stab/Kick)
  (bind (_outhit _returnvalue_2) (Collision|SphereTraceByChannel _returnvalue _returnvalue 25.0 "TraceTypeQuery1" false 0 "ForDuration"))
  (if _returnvalue_2
    (if (Actor|ActorHasTag (.HitActor (Collision|BreakHitResult _outhit)) "Damageable")
      (Game|Damage|ApplyDamage (.HitActor (Collision|BreakHitResult _outhit)) 1e+01 0 0)
      (Camera|PlayWorldCameraShake "/Game/Blueprints/BP_SwordHitCameraShake.BP_SwordHitCameraShake_C" (.Location (Collision|BreakHitResult _outhit)) 0.0 2e+03)
      (CallFunction|PlaySwordHitSounds)
      (Effects|SpawnEmitteratLocation "/Game/VFXs/Particles/Blood/P_Blood_Splat_Cone.P_Blood_Splat_Cone" (.Location (Collision|BreakHitResult _outhit)) (Math|Rotator|MakeRotfromXY (.Normal (Collision|BreakHitResult _outhit)) (.ImpactNormal (Collision|BreakHitResult _outhit))) "0.400000,0.400000,0.400000" true "AutoRelease"))))

(event Custom|Play%20Sword%20Hit%20Sounds
  ;[0.05127 0.05127 0.05127] Play Sword Hit Sounds
  (Audio|PlaySoundatLocation "/Game/Sounds/Sword_Hits/MS_SwordHit.MS_SwordHit" (Transformation|GetActorLocation (Components|GetOwner)) "0, 0, 0" 1.0 1.0 0.0 "/Game/Sounds/SA_Character.SA_Character" 0 0 0))

(event Custom|Ragdoll
  ;[0.05127 0.05127 0.05127] Enable Ragdoll
  (Utilities|FlowControl|Delay 2.0)
  (Physics|SetSimulatePhysics (Variables|Character|GetMesh) true)
  (Audio|PlaySoundatLocation "/Game/Sounds/Grunts-Hits/Death_1.Death_1" (Transformation|GetActorLocation) "0, 0, 0" 1.0 1.0 0.0 "/Game/Sounds/SA_Character.SA_Character" 0 0 0))

(event Custom|Begin%20Combo%20Attack%20AI
  ;[0.05127 0.05127 0.05127] Combo System
  ;;[0.05127 0.05127 0.05127] Attack Input
  (if (Variables|Attack|GetCanAttack)
    (CallFunction|SwordAttack)))

(event Custom|StopCombo
  ;[0.05127 0.05127 0.05127] Combo System
  ;;[0.05127 0.05127 0.05127] Stop Combo/Attack
  (Variables|Attack|SetIsAttacking false)
  (Variables|Attack|SetAttackIndex 0))

(event Custom|Attack%202
  ;[0.05127 0.05127 0.05127] Combo System
  ;;[0.05127 0.05127 0.05127] Attack 2
  (Utilities|FlowControl|DoOnce false :!label _label
    (:Completed
      (Utilities|FlowControl|Delay 0.1)
      (Animation|Montage|PlayMontage (Variables|Character|GetMesh) "/Game/Animations/Sword_Attacks/Attack2_Montage.Attack2_Montage" (Variables|Default|GetAttackAnimationRate)
        (:then
          (Variables|Attack|SetAttackIndex 2)
          (goto _label Reset))))))

(event Custom|Attack%201
  ;[0.05127 0.05127 0.05127] Combo System
  ;;[0.05127 0.05127 0.05127] Attack 1
  (Utilities|FlowControl|DoOnce false :!label _label
    (:Completed
      (Utilities|FlowControl|Delay 0.1)
      (Animation|Montage|PlayMontage (Variables|Character|GetMesh) "/Game/Animations/Sword_Attacks/Attack1_Montage.Attack1_Montage" (Variables|Default|GetAttackAnimationRate)
        (:then
          (Variables|Attack|SetAttackIndex 1)
          (goto _label Reset))))))

(event Custom|Start%20Sword%20Trace
  ;[0.05127 0.05127 0.05127] Sword Trace
  (bind _returnvalue (Utilities|Time|SetTimerbyEvent (delegate Custom|Sword%20Trace%20Loop) 0.016 true))
  (Variables|Default|SetSwordTraceLoop _returnvalue))

(event Custom|Attack%204
  ;[0.05127 0.05127 0.05127] Combo System
  ;;[0.05127 0.05127 0.05127] Attack 4
  (Utilities|FlowControl|DoOnce false :!label _label
    (:Completed
      (Utilities|FlowControl|Delay 0.1)
      (Animation|Montage|PlayMontage (Variables|Character|GetMesh) "/Game/Animations/Sword_Attacks/Attack3_Montage.Attack3_Montage" (Variables|Default|GetAttackAnimationRate)
        (:then
          (Variables|Attack|SetAttackIndex 4)
          (goto _label Reset))))))

(event Custom|Enable/Disable%20Investigation%20Icon
  (bind _investigationwidget (Variables|Default|GetInvestigationWidget))
  (Utilities|FlowControl|FlipFlop
    (:A
      (Rendering|SetVisibility _investigationwidget true false))
    (:B
      (Rendering|SetVisibility _investigationwidget false false))))

(event Custom|Sword%20Trace%20Loop
  ;[0.05127 0.05127 0.05127] Sword Trace
  (bind (_outhit _returnvalue) (Collision|SphereTraceByChannel (Transformation|GetWorldLocation (Variables|Default|GetSword%20Top%20Point)) (Transformation|GetWorldLocation (Variables|Default|GetSword%20Bottom%20Point)) 12.0 "TraceTypeQuery1" false 0 "ForDuration" true "(R=1.000000,G=0.000000,B=0.000000,A=1.000000)" "(R=0.000000,G=1.000000,B=0.000000,A=1.000000)" 0.2))
  (if _returnvalue
    (if (Actor|ActorHasTag (.HitActor (Collision|BreakHitResult _outhit)) "Damageable")
      (Utilities|FlowControl|DoOnce false :!label _label
        (:Completed
          (Game|Damage|ApplyDamage (.HitActor (Collision|BreakHitResult _outhit)) 1e+01 0 0)
          (CallFunction|PlaySwordHitSounds)
          (Camera|PlayWorldCameraShake "/Game/Blueprints/BP_SwordHitCameraShake.BP_SwordHitCameraShake_C" (.Location (Collision|BreakHitResult _outhit)) 0.0 2e+03)
          (Effects|SpawnEmitteratLocation "/Game/VFXs/Particles/Blood/P_Blood_Splat_Cone.P_Blood_Splat_Cone" (.Location (Collision|BreakHitResult _outhit)) (Math|Rotator|MakeRotfromXY (.Normal (Collision|BreakHitResult _outhit)) (.Normal (Collision|BreakHitResult _outhit))) "0.400000,0.400000,0.400000" true "AutoRelease")
          (Utilities|FlowControl|Delay 0.5)
          (goto _label Reset))))))

(event Custom|Stop%20Sword%20Trace
  ;[0.05127 0.05127 0.05127] Sword Trace
  (Utilities|Time|ClearandInvalidateTimerbyHandle (Variables|Default|GetSwordTraceLoop)))

(event EventTick
  (params (DeltaSeconds :type Float%20%28single-precision%29))
  (bind _assassinate_widget (Variables|Default|GetAssassinate%20Widget))
  (bind _investigationwidget (Variables|Default|GetInvestigationWidget))
  (bind _dummyhud (Variables|Default|GetDummyHUD))
  ;[0.05127 0.05127 0.05127] Rotate UI Towards Character
  (bind _final_rotation (CallFunction|SetUIRotation _dummyhud))
  (Transformation|SetWorldRotation _dummyhud _final_rotation false false)
  (bind _final_rotation_2 (CallFunction|SetUIRotation _assassinate_widget))
  (Transformation|SetWorldRotation _assassinate_widget _final_rotation_2 false false)
  (bind _final_rotation_3 (CallFunction|SetUIRotation _investigationwidget))
  (Transformation|SetWorldRotation _investigationwidget _final_rotation_3 false false))

(event EventBeginPlay
  ;[0.05127 0.05127 0.05127] Create Widget
  (bind _aswb_dummy_hud (Utilities|Casting|CastToWB_Dummy_HUD (UserInterface|GetWidget (Variables|Default|GetDummyHUD))))
  (Variables|Default|SetDummyUI _aswb_dummy_hud)
  (Default|InitDummyData (Variables|Default|GetBP_PlayerStats)))

(event Game|Damage|EventAnyDamage
  (params (Damage :type Float%20%28single-precision%29) (DamageType :type Damage%20Type%20Object%20Reference) (InstigatedBy :type Controller%20Object%20Reference) (DamageCauser :type Actor%20Object%20Reference))
  (bind _hitanims (Variables|Default|GetHitAnims))
  ;[0.05127 0.05127 0.05127] Take Hit
  (if (not (Variables|Default|GetIsPlayerDead))
    (CallFunction|StopCombo)
    (Animation|PlayAnimMontage (Utilities|Array|Get(acopy) _hitanims (Math|Random|RandomIntegerinRange 0 (- (Utilities|Array|Length _hitanims) 1))) 1.0 "None")
    (bind _asbp_third_person_character (Utilities|Casting|CastToBP_ThirdPersonCharacter (Game|GetPlayerCharacter 0)))
    (Character|LaunchCharacter (* (Math|Vector|GetForwardVector (Transformation|GetActorRotation _asbp_third_person_character)) 7e+02) false false)
    (Audio|PlaySoundatLocation "/Game/Sounds/Grunts-Hits/Death_2.Death_2" (Transformation|GetActorLocation) "0, 0, 0" 1.0 (Math|Random|RandomFloatinRange 0.8 1.2) 0.0 "/Game/Sounds/SA_Character.SA_Character" 0 0 0)
    (bind _isplayerdead (Default|DecreaseHealth (Variables|Default|GetBP_PlayerStats) Damage))
    (Variables|Default|SetIsPlayerDead _isplayerdead)
    (if _isplayerdead
      (Collision|SetCollisionObjectType (Variables|Character|GetMesh) "ECC_PhysicsBody")
      (CallFunction|Ragdoll)
      (Rendering|SetVisibility (Variables|Default|GetDummyHUD) false false)
      (Rendering|SetVisibility (Variables|Default|GetAssassinate%20Widget) false false)
      (Variables|/Game/Blueprints/Characters/BP_ThirdPersonCharacter.BP_ThirdPersonCharacter_C|SetActorToLockOn _asbp_third_person_character 0)
      (Utilities|FlowControl|Delay 2.0)
      (Collision|SetCollisionEnabled (Variables|Collision|GetCapsuleComponent) "NoCollision"))))

(fn ConstructionScript)

(fn SetUIRotation
  (params (Widget :type Widget%20Component%20Object%20Reference))
  (return (Math|Rotator|FindLookatRotation (Transformation|GetWorldLocation Widget) (Transformation|GetWorldLocation (Variables|/Script/Engine.PlayerCameraManager|GetTransformComponent (Game|GetPlayerCameraManager 0))))))

(fn Attack
  (CallFunction|BeginComboAttackAI)
  (return 0.4))

(fn StealthBackAssassin
  (Animation|PlayAnimMontage "/Game/Animations/Assassinations/Paired_Knife_Stealth_KidneyAndNeck_Vic_Montage.Paired_Knife_Stealth_KidneyAndNeck_Vic_Montage" 1.0 "None")
  (CallFunction|Ragdoll)
  (Rendering|SetVisibility (Variables|Default|GetAssassinate%20Widget) false false)
  (return (Transformation|GetWorldLocation (Variables|Default|GetAssassin%20REF)) (Transformation|GetActorRotation)))